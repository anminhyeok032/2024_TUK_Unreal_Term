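; BP_Door01 is a sliding door that rises and lowers in response to BP_Button_01 actors, whose push and release events it binds at BeginPlay.
; A push plays a timeline that raises the mesh below a fixed height cap, recording a floor height on first movement.
; Release waits briefly, then a second timeline lowers it toward that floor.
; Flags limit open and close sounds, resetting when movement hits a limit.
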(event OnComponentEndOverlap(Front)
  (params (OverlappedComponent :type Primitive%20Component%20Object%20Reference) (OtherActor :type Actor%20Object%20Reference) (OtherComp :type Primitive%20Component%20Object%20Reference) (OtherBodyIndex :type Integer)))

(event Custom|ButtonP
  (bind _returnvalue (Transformation|GetActorLocation))
  (if true
    (bind _door (Timeline|Timeline PlayFromStart)
      (:Update
        (if (> 7e+02 (+ (.z _returnvalue) _door))
          (Transformation|SetRelativeLocation (Variables|Debug|GetStaticMeshComponent) (Math|Vector|MakeVector (.x _returnvalue) (.y _returnvalue) (+ (.z _returnvalue) _door)) false false)
          (Variables|Default|SetDoorZ (+ (.z _returnvalue) _door))
          (if (not (Variables|Default|GetOpenSound))
            (Audio|PlaySoundatLocation "/Game/BPs/Sounds/portal_2_door_open.portal_2_door_open" (Transformation|GetActorLocation) "0, 0, 0" 1.0 1.0 0.0 0 0 0 0)
            (Variables|Default|SetOpenSound true)
            (Variables|Default|SetDoorFirst (.z _returnvalue)))
          (else
            (Variables|Default|SetOpenSound false)))))))

(event Custom|EndButton
  (bind _returnvalue (Transformation|GetActorLocation))
  (Utilities|FlowControl|Delay 1.0)
  (bind _door (Timeline|Timeline_0 PlayFromStart)
    (:Update
      (if (> 7e+02 (- (.z _returnvalue) _door))
        (if (> (- (.z _returnvalue) _door) (Variables|Default|GetDoorFirst))
          (Transformation|SetRelativeLocation (Variables|Debug|GetStaticMeshComponent) (Math|Vector|MakeVector (.x _returnvalue) (.y _returnvalue) (- (.z _returnvalue) _door)) false false)
          (if (not (Variables|Default|GetCloseSound))
            (Audio|PlaySoundatLocation "/Game/BPs/Sounds/portal_2_door_close.portal_2_door_close" (Transformation|GetActorLocation) "0, 0, 0" 1.0 1.0 0.0 0 0 0 0)
            (Variables|Default|SetCloseSound true))
          (else
            (Variables|Default|SetCloseSound false)))))))

(event EventBeginPlay
  (bind _outactors (Actor|GetAllActorsOfClass "/Game/BPs/Button/BP_Button_01.BP_Button_01_C"))
  (EventDispatchers|BindEventtoPush _outactors (delegate Custom|ButtonP))
  (EventDispatchers|BindEventtoEndPush _outactors (delegate Custom|EndButton)))

(event Collision|EventActorBeginOverlap
  (params (OtherActor :type Actor%20Object%20Reference)))

(event EventTick
  (params (DeltaSeconds :type Float%20%28single-precision%29)))

(fn ConstructionScript)

(fn Level01Button
  (params (Push :type Boolean))
  (return false))